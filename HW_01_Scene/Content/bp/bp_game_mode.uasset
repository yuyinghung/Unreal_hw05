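; Game mode Blueprint that runs a minutes-and-seconds countdown and pauses the game when time runs out.
; Event Tick feeds a one-second Delay, which throttles the decrement of Sec to roughly once per second.
; When Sec drops below zero it wraps to 59 and borrows from Min.
; With no minutes left, Sec resets to zero and the game pauses.
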(event `self.ReceiveTick`
  (params (DeltaSeconds :type "Float (single-precision)"))
  ;[1 0 0] countdown system
  ;;[1 1 1] 每秒秒數減一
  (`KismetSystemLibrary.Delay` 1.0) ; delay:wait for the chosen timing to execute the afterwards target
  (bind _output_get (set `self.sec` (- (`self.sec`) 1)))
  ;;[1 1 1] 當秒數低於零就把秒數設定為59
  (if (< _output_get 0)
    (set `self.sec` 59)
    ;;[1 1 1] 分大於0時減一
    (if (> (`self.min`) 0)
      (set `self.min` (- (`self.min`) 1))
      (else
        ;;[1 1 1] 分為0時酩等於59就代表已經沒時間.將秒設為0並暫停遊戲
        (if (== (`self.sec`) 59)
          (set `self.sec` 0)
          (`GameplayStatics.SetGamePaused` true))))))

(fn `UserConstructionScript`)